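; Actor component that pushes its physics-simulated owner with sail wind while the player character is in a boat.
; BeginPlay caches the wind controller, the owner's root primitive and the player, disabling tick if no controller exists.
; With sail up and positive DynamicWindScale, Tick applies delta-time-scaled force from the wind-to-sail dot product, plus yaw torque signed by their cross product.
; AddWindScale adjusts DynamicWindScale, which only gates the effect.
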(event `self.ReceiveBeginPlay`
  (bind _returnvalue (`GameplayStatics.GetActorOfClass` "/Game/Wind/BP_WindController.BP_WindController_C"))
  (`/Engine/EditorBlueprintResources/StandardMacros.IsValid` _returnvalue
    (:`Is Valid`
      (set `self.wind controller` _returnvalue)
      (bind _asprimitive_component (cast `PrimitiveComponent` (`Actor.RootComponent` (`self.GetOwner`))))
      (set `self.As Primitive Component` _asprimitive_component)
      (bind _returnvalue_2 (`GameplayStatics.GetActorOfClass` "/Game/FirstPerson/Blueprints/BP_FirstPersonCharacter.BP_FirstPersonCharacter_C"))
      (set `self.person` _returnvalue_2))
    (:`Is Not Valid`
      (`self.SetComponentTickEnabled` false))))

(event `self.ReceiveTick`
  (params (DeltaSeconds :type "Float (single-precision)"))
  (bind _person (`self.person`))
  (bind _as_primitive_component (`self.As Primitive Component`))
  (bind _wind_controller (`self.wind controller`))
  (bind _returnvalue (`SceneComponent.K2_GetComponentLocation` _as_primitive_component))
  (bind _windvector (`/Game/Wind/BP_WindController.WindVector` _wind_controller))
  (bind _returnvalue_2 (`KismetMathLibrary.Normal` _windvector))
  (bind (_returnvalue_roll _returnvalue_pitch _returnvalue_yaw) (`KismetMathLibrary.BreakRotator` (`KismetMathLibrary.FindLookAtRotation` _returnvalue (+ _returnvalue _windvector))))
  (bind _returnvalue_3 (`KismetMathLibrary.Normal` (`SceneComponent.GetForwardVector` (`/Game/Blueprints/BP_boat.sail` (`/Game/FirstPerson/Blueprints/BP_FirstPersonCharacter.ControlBoat` (`self.person`))))))
  (bind (_returnvalue_x _returnvalue_y _returnvalue_z) (`KismetMathLibrary.BreakVector` (`KismetMathLibrary.Cross_VectorVector` _returnvalue_2 _returnvalue_3)))
  (if (`KismetSystemLibrary.IsValid` _person)
    (if (`/Game/FirstPerson/Blueprints/BP_FirstPersonCharacter.inBoat` _person)
      (if (> (`self.dynamic wind scale`) 0.0)
        (if (`SceneComponent.IsSimulatingPhysics` (`self.As Primitive Component`) "None")
          (if (`KismetSystemLibrary.IsValid` _wind_controller)
            (if (`self.SailUp`)
              (`PrimitiveComponent.AddForce` _as_primitive_component (* (`KismetMathLibrary.Dot_VectorVector` _returnvalue_2 _returnvalue_3) _windvector (* (/ 60.0 (/ 1.0 (`GameplayStatics.GetWorldDeltaSeconds`))) 1.8) 1000.0) "None" true)
              (if (`KismetMathLibrary.NearlyEqual_FloatFloat` 0.0 _returnvalue_yaw 5.0)
                _
                (elif (`self.SailUp`)
                  (`PrimitiveComponent.AddTorqueInDegrees` (`self.As Primitive Component`) (`KismetMathLibrary.MakeVector` 0.0 0.0 (* (`KismetMathLibrary.SelectFloat` -18.0 18.0 (> _returnvalue_z 0.0)) (`self.base wind scale`) (/ 60.0 (/ 1.0 (`GameplayStatics.GetWorldDeltaSeconds`))))) "None" true))))))))))

(fn `Add wind scale`
  (params (A :type "Float (double-precision)"))
  (set `self.dynamic wind scale` (`KismetMathLibrary.FClamp` (+ A (`self.dynamic wind scale`)) 0.0 100000.0)))